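; Game mode for the space shooter that tracks kills and level progression and relays player death to the HUD.
; PlayerDead forwards the event to the HUD Blueprint.
; EnemyDead increments the destroyed count, sets Progress one above that count, and raises Level on every third kill.
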(event `self.ReceiveTick`
  (params (DeltaSeconds :type "Float (single-precision)")))

(event `PlayerDead`
  (`/Game/SpaceShooter/Bluprints/BP_Hud.PlayerDead` (`self.BP_Hud`)))

(event `EnemyDead`
  (bind _returnvalue (+ (`self.EnemiesDestroyed`) 1))
  (bind _output_get (set `self.EnemiesDestroyed` _returnvalue))
  (set `self.Progress` _returnvalue)
  (if (== (mod _output_get 3) 0)
    (set `self.Level` (+ (`self.Level`) 1))))

(fn `UserConstructionScript`)