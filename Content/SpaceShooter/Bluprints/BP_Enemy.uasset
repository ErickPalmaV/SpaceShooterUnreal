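; Enemy actor for a space shooter that flies straight along its initial forward vector while firing from two spawn points.
; Tick moves it without sweep and spawns the Ammo class in pairs, gated by a FireRate cooldown.
; Overlapping an actor tagged "Player" fires OnEnemyDestroy once, notifying BP_GameMode via EnemyDead and destroying the enemy after a short delay.
; A BulletPlayer cast into that death logic is left unconnected.
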(event `self.ReceiveBeginPlay`
  (set `self.MovemenVector` (`self.GetActorForwardVector`))
  (add `self.OnEnemyDestroy` (delegate `Destroyed_Event`)))

(event `Destroyed_Event`
  (`KismetSystemLibrary.Delay` 0.2)
  (`self.K2_DestroyActor`))

(event `self.ReceiveTick`
  (params (DeltaSeconds :type "Float (single-precision)"))
  (`self.Movement` DeltaSeconds)
  (if (`self.CanShoot`)
    (`self.Shoot` (`self.ammo`))
    (`self.CoolDownShoot`)))

(event `CoolDownShoot`
  (set `self.CanShoot` false)
  (`KismetSystemLibrary.Delay` (`self.FireRate`))
  (set `self.CanShoot` true))

(event `self.ReceiveActorBeginOverlap`
  (params (OtherActor :type "Actor Object Reference"))
  (if (`KismetArrayLibrary.Array_Contains` (`Actor.Tags` OtherActor) "Player")
    (if (`self.CanBeDamage`)
      (`self.OnEnemyDestroy`)
      (set `self.CanBeDamage` false)
      (bind _asbp_game_mode (cast `/Game/SpaceShooter/Bluprints/BP_GameMode` (`GameplayStatics.GetGameMode`)))
      (`/Game/SpaceShooter/Bluprints/BP_GameMode.EnemyDead` _asbp_game_mode))))

(fn `Movement`
  (params (DeltaSecods :type "Float (double-precision)"))
  (`self.K2_SetActorLocation` (+ (`self.K2_GetActorLocation`) (* (* DeltaSecods (`self.speed`)) (`self.MovemenVector`)))))

(fn `Shoot`
  (params (ammo :type "Actor Class Reference"))
  (`|SpawnActorFromClass` ammo (`SceneComponent.K2_GetComponentToWorld` (`self.SpawnPoint1`)) "Undefined" "MultiplyWithRoot" null null)
  (`|SpawnActorFromClass` ammo (`SceneComponent.K2_GetComponentToWorld` (`self.SpawnPoint2`)) "Undefined" "MultiplyWithRoot" null null))

(fn `UserConstructionScript`)