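; Enemy spawner actor for the space shooter that spawns enemies on a looping timer set by SpawnTime.
; Each spawn picks a random SceneComponent tagged "SpawnPoint" on the actor and uses its world transform.
; The enemy class is a random index below the GameMode's Level, clamped by MaxEnemies, choosing BP_Enemy or BP_EnemyH, so higher levels can widen the mix.
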(event `self.ReceiveBeginPlay`
  (`KismetSystemLibrary.K2_SetTimerDelegate` (delegate `Spawn`) (`self.SpawnTime`) true)
  (bind _asbp_game_mode (cast `/Game/SpaceShooter/Bluprints/BP_GameMode` (`GameplayStatics.GetGameMode`)))
  (set `self.GameMode` _asbp_game_mode))

(event `Spawn`
  (bind _enemt_spawned (`self.SpawnEnemy`))
  (cast `/Game/SpaceShooter/Bluprints/BP_Enemy` _enemt_spawned))

(fn `GetClassToSpawn`
  (params (Type :type Integer))
  (returns (Class :type "Actor Class Reference"))
  (return (select `int` (`KismetMathLibrary.Clamp` Type 0 (- (`self.MaxEnemies`) 1)) :`0` "/Game/SpaceShooter/Bluprints/BP_Enemy.BP_Enemy_C" :`1` "/Game/SpaceShooter/Bluprints/BP_EnemyH.BP_EnemyH_C" :!type "/Game/SpaceShooter/Bluprints/BP_Enemy Class Reference")))

(fn `SpawnEnemy`
  (returns (`Enemt Spawned` :type "/Game/SpaceShooter/Bluprints/BP_Enemy Object Reference"))
  (bind _returnvalue (`self.GetComponentsByTag` "/Script/Engine.SceneComponent" "SpawnPoint"))
  (bind _class (`self.GetClassToSpawn` (`KismetMathLibrary.RandomInteger` (`/Game/SpaceShooter/Bluprints/BP_GameMode.Level` (`self.GameMode`)))))
  (bind _returnvalue_2 (`|SpawnActorFromClass` _class (`SceneComponent.K2_GetComponentToWorld` (`|GetArrayItem` _returnvalue (`KismetMathLibrary.RandomInteger` (`KismetArrayLibrary.Array_Length` _returnvalue)))) "Undefined" "MultiplyWithRoot" null null))
  (bind _asbp_enemy (cast `/Game/SpaceShooter/Bluprints/BP_Enemy` _returnvalue_2))
  (return _asbp_enemy))

(fn `UserConstructionScript`)